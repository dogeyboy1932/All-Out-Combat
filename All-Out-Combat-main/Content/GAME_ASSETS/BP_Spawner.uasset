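; Enemy spawner that periodically spawns level-specific AI enemies at random X/Y offsets around the player hero.
; On BeginPlay it reads the level from GlobalVars and starts a looping spawn timer using that object's spawn interval.
; Level-checked functions spawn roaming pursuers, shooters or exploders for levels one to three.
; Level three's timer calls the level-two function SpawnEnemy2, so the exploder function SpawnEnemy3 is never triggered here.
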(event EventBeginPlay
  ;[0.15 0.15 0.15 0.5] Spawning Enemies
  (bind _asglobal_vars (Utilities|Casting|CastToGlobalVars (Game|GetGameInstance)))
  (if (== (Variables|/Game/GAME_ASSETS/GlobalVars.GlobalVars_C|GetCurrentLevel _asglobal_vars) 1)
    (bind _asglobal_vars_2 (Utilities|Casting|CastToGlobalVars (Game|GetGameInstance)))
    (Utilities|Time|SetTimerbyFunctionName 0 "SpawnEnemy" (Variables|/Game/GAME_ASSETS/GlobalVars.GlobalVars_C|GetTimeBetweenSpawns _asglobal_vars_2) true)
    (elif (== (Variables|/Game/GAME_ASSETS/GlobalVars.GlobalVars_C|GetCurrentLevel _asglobal_vars) 2)
      (bind _asglobal_vars_3 (Utilities|Casting|CastToGlobalVars (Game|GetGameInstance)))
      (Utilities|Time|SetTimerbyFunctionName 0 "SpawnEnemy2" (Variables|/Game/GAME_ASSETS/GlobalVars.GlobalVars_C|GetTimeBetweenSpawns _asglobal_vars_3) true)
      (elif (== (Variables|/Game/GAME_ASSETS/GlobalVars.GlobalVars_C|GetCurrentLevel _asglobal_vars) 3)
        (bind _asglobal_vars_4 (Utilities|Casting|CastToGlobalVars (Game|GetGameInstance)))
        (Utilities|Time|SetTimerbyFunctionName 0 "SpawnEnemy2" (Variables|/Game/GAME_ASSETS/GlobalVars.GlobalVars_C|GetTimeBetweenSpawns _asglobal_vars_4) true)))))

(fn ConstructionScript)

(fn SpawnEnemy
  ;[0.15 0.15 0.15 0.5] Spawning Pursuer (Level One)
  (bind _asglobal_vars (Utilities|Casting|CastToGlobalVars (Game|GetGameInstance)))
  (if (== (Variables|/Game/GAME_ASSETS/GlobalVars.GlobalVars_C|GetCurrentLevel _asglobal_vars) 1)
    (bind _asbp_hero (Utilities|Casting|CastToBP_Hero (Game|Player|GetPlayerPawn 0)))
    (bind _returnvalue (AI|SpawnAIFromClass "/Game/GAME_ASSETS/Enemies/BP_Basic_Pursuer_Enemy.BP_Basic_Pursuer_Enemy_C" 0 (Math|Vector|MakeVector (+ (.x (Transformation|GetActorLocation _asbp_hero)) (Math|Random|RandomFloatinRange -1e+03 1e+03)) (+ (.y (Transformation|GetActorLocation _asbp_hero)) (Math|Random|RandomFloatinRange -1e+03 1e+03)) (.z (Transformation|GetActorLocation _asbp_hero))) "0, 0, 0" false 0))
    (bind _asbp_basic_pursuer_enemy (Utilities|Casting|CastToBP_Basic_Pursuer_Enemy _returnvalue))
    (Default|Roam _asbp_basic_pursuer_enemy)))

(fn SpawnEnemy2
  ;[0.15 0.15 0.15 0.5] Spawning Shooter (Level Two)
  (bind _asglobal_vars (Utilities|Casting|CastToGlobalVars (Game|GetGameInstance)))
  (if (== (Variables|/Game/GAME_ASSETS/GlobalVars.GlobalVars_C|GetCurrentLevel _asglobal_vars) 2)
    (bind _asbp_hero (Utilities|Casting|CastToBP_Hero (Game|Player|GetPlayerPawn 0)))
    (AI|SpawnAIFromClass "/Game/GAME_ASSETS/Enemies/Shooters.Shooters_C" 0 (Math|Vector|MakeVector (+ (.x (Transformation|GetActorLocation _asbp_hero)) (Math|Random|RandomFloatinRange -1e+03 1e+03)) (+ (.y (Transformation|GetActorLocation _asbp_hero)) (Math|Random|RandomFloatinRange -1e+03 1e+03)) (.z (Transformation|GetActorLocation _asbp_hero))) "0, 0, 0" false 0)))

(fn SpawnEnemy3
  ;[0.15 0.15 0.15 0.5] Spawning Pursuer (Level One)
  (bind _asglobal_vars (Utilities|Casting|CastToGlobalVars (Game|GetGameInstance)))
  (if (== (Variables|/Game/GAME_ASSETS/GlobalVars.GlobalVars_C|GetCurrentLevel _asglobal_vars) 3)
    (bind _asbp_hero (Utilities|Casting|CastToBP_Hero (Game|Player|GetPlayerPawn 0)))
    (AI|SpawnAIFromClass "/Game/GAME_ASSETS/Enemies/Exploders.Exploders_C" 0 (Math|Vector|MakeVector (+ (.x (Transformation|GetActorLocation _asbp_hero)) (Math|Random|RandomFloatinRange -1e+03 1e+03)) (+ (.y (Transformation|GetActorLocation _asbp_hero)) (Math|Random|RandomFloatinRange -1e+03 1e+03)) (.z (Transformation|GetActorLocation _asbp_hero))) "0, 0, 0" false 0)))