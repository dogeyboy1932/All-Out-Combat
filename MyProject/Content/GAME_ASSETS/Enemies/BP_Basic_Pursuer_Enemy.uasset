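; BP_Basic_Pursuer_Enemy is an enemy that roams, chases the hero and dies to a single bullet.
; Roam loops random reachable moves, while PawnSensing starts an AI move toward the hero and calls Roam two seconds after issuing it.
; Capsule hits on the hero deal damage and knockback, briefly disabling the enemy's movement.
; Bullet overlap adds coins to GlobalVars, updates the score GUI and destroys both actors.
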(event OnSeePawn(PawnSensing)
  (params (Pawn :type Pawn%20Object%20Reference))
  ;[0.15 0.15 0.15 0.5] Player Sensing
  (bind _asbp_hero (Utilities|Casting|CastToBP_Hero (Game|GetPlayerCharacter 0)))
  (AI|AIMoveTo self "0, 0, 0" _asbp_hero 7e+01 false
    (:then
      (Utilities|FlowControl|Delay 2.0)
      (CallFunction|Roam))))

(event OnComponentHit(CapsuleComponent)
  (params (HitComponent :type Primitive%20Component%20Object%20Reference) (OtherActor :type Actor%20Object%20Reference) (OtherComp :type Primitive%20Component%20Object%20Reference) (NormalImpulse :type Vector :default "0, 0, 0") (Hit :type Hit%20Result%20Structure%20%28by%20ref%29))
  (bind _returnvalue (* NormalImpulse -1e+03))
  (bind (_x _y _z) (Math|Vector|BreakVector _returnvalue))
  ;[0.15 0.15 0.15 0.5] Damaging Player
  (bind _asbp_hero (Utilities|Casting|CastToBP_Hero OtherActor))
  (Character|LaunchCharacter _asbp_hero (Math|Vector|MakeVector (+ _x 3e+02) (+ _y 4e+02) (+ _z 3e+02)) false false)
  (Game|Damage|ApplyDamage _asbp_hero 1e+01 0 0)
  (Pawn|Components|CharacterMovement|DisableMovement (Variables|Character|GetCharacterMovement))
  (Utilities|FlowControl|Delay 1.5)
  (Pawn|Components|CharacterMovement|SetMovementMode (Variables|Character|GetCharacterMovement) "MOVE_Walking" 0)
  (CallFunction|Roam))

(event OnComponentBeginOverlap(CapsuleComponent)
  (params (OverlappedComponent :type Primitive%20Component%20Object%20Reference) (OtherActor :type Actor%20Object%20Reference) (OtherComp :type Primitive%20Component%20Object%20Reference) (OtherBodyIndex :type Integer) (bFromSweep :type Boolean) (SweepResult :type Hit%20Result%20Structure%20%28by%20ref%29))
  (bind _asbp_bullet (Utilities|Casting|CastToBP_Bullet OtherActor))
  (bind _asglobal_vars (Utilities|Casting|CastToGlobalVars (Game|GetGameInstance)))
  (bind _output_get (Variables|/Game/GAME_ASSETS/GlobalVars.GlobalVars_C|SetCoins _asglobal_vars (+ (Variables|/Game/GAME_ASSETS/GlobalVars.GlobalVars_C|GetCoins _asglobal_vars) (Variables|Default|GetCoinsWorth))))
  (Default|SetCoinsText (Variables|/Game/GAME_ASSETS/GlobalVars.GlobalVars_C|GetScoreGUI _asglobal_vars) _output_get)
  (Actor|DestroyActor _asbp_bullet)
  (Actor|DestroyActor))

(event Custom|Roam
  ;[0.15 0.15 0.15 0.5] Roaming Functionality
  (AI|AIMoveTo self (.RandomLocation (AI|Navigation|GetRandomReachablePointinRadius (Transformation|GetActorLocation) 1e+03 0 0)) 0 5.0 false
    (:OnSuccess
      (Utilities|FlowControl|Delay 2.0)
      (CallFunction|Roam))))

(event EventBeginPlay
  (CallFunction|Roam))

(event Collision|EventActorBeginOverlap
  (params (OtherActor :type Actor%20Object%20Reference)))

(event EventTick
  (params (DeltaSeconds :type Float%20%28single-precision%29)))

(fn ConstructionScript)

(fn RoamFunc
  (CallFunction|Roam))