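; Enemy spawner that periodically creates basic pursuer enemies around the player's hero.
; On BeginPlay it starts a looping SpawnEnemy timer, with the interval read from the GlobalVars game instance.
; SpawnEnemy uses SpawnAIFromClass at a random X/Y offset from the hero, at the hero's height, then prints a debug message.
; A SpawnActor alternative and a Roam call remain in the graph but never run.
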(event EventBeginPlay
  (bind _asglobal_vars (Utilities|Casting|CastToGlobalVars (Game|GetGameInstance)))
  (Utilities|Time|SetTimerbyFunctionName 0 "SpawnEnemy" (Variables|/Game/GAME_ASSETS/GlobalVars.GlobalVars_C|GetTimeBetweenSpawns _asglobal_vars) true))

(event Collision|EventActorBeginOverlap
  (params (OtherActor :type Actor%20Object%20Reference)))

(event EventTick
  (params (DeltaSeconds :type Float%20%28single-precision%29)))

(fn ConstructionScript)

(fn SpawnEnemy
  (bind _asbp_hero (Utilities|Casting|CastToBP_Hero (Game|Player|GetPlayerPawn 0)))
  (bind _returnvalue (AI|SpawnAIFromClass "/Game/GAME_ASSETS/Enemies/BP_Basic_Pursuer_Enemy.BP_Basic_Pursuer_Enemy_C" 0 (Math|Vector|MakeVector (+ (.x (Transformation|GetActorLocation _asbp_hero)) (Math|Random|RandomFloatinRange -1e+03 1e+03)) (+ (.y (Transformation|GetActorLocation _asbp_hero)) (Math|Random|RandomFloatinRange -1e+03 1e+03)) (.z (Transformation|GetActorLocation _asbp_hero))) "0, 0, 0" false 0))
  (bind _asbp_basic_pursuer_enemy (Utilities|Casting|CastToBP_Basic_Pursuer_Enemy _returnvalue))
  (Development|PrintString "Enemy spawned"))